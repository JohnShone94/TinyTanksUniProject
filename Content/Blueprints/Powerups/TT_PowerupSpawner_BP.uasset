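; Tiny Tanks spawner that periodically drops powerups onto random empty world grid cells during a match.
; From BeginPlay, a self-looping five-second Delay checks that the game has started, the count is below four and a coin flip passes.
; It marks the cell filled, spawns a scaled-up powerup above it and increments the count, which PowerupsTake decrements.
; The loop does not re-arm when no valid empty cell is returned.
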(event Custom|PowerupsTake
  (Variables|Default|SetNoPowerups (- (Variables|Default|GetNoPowerups) 1)))

(event EventBeginPlay
  (bind _astt_tiny_tanks_game_mode (Utilities|Casting|CastToTT_TinyTanksGameMode (Game|GetGameMode)))
  (Utilities|FlowControl|Delay 5.0 :!label _label)
  (if (Class|TTTinyTanksGameMode|GetGameStarted _astt_tiny_tanks_game_mode)
    (Math|Integer|CompareInt (Variables|Default|GetNoPowerups) 4
      (:==
        (goto _label))
      (:<
        (if (Math|Random|RandomBoolwithWeight 0.5)
          (bind _outactors (Actor|GetAllActorsOfClass "/Script/TinyTanksUniProject.TT_WorldGrid"))
          (for _array_element _outactors
            (bind _returnvalue (Class|TTWorldGrid|GetRandomEmptyCell _array_element))
            (Utilities|IsValid _returnvalue
              (:Is%20Valid
                (Class|TTGridCell|SetCellFilled _returnvalue true)
                (Game|SpawnActorfromClass "/Game/Blueprints/Powerups/TT_Powerup_BP.TT_Powerup_BP_C" (Math|Transform|MakeTransform (+ (Transformation|GetActorLocation _returnvalue) "0,0,55.000000") "0, 0, 0" "2.000000,2.000000,2.000000") "Undefined" 0 0)
                (Math|Integer|IncrementInt (Variables|Default|GetNoPowerups)
                  (:%20%20
                    (goto _label))))))
          (else
            (goto _label)))))
    (else
      (goto _label))))

(fn ConstructionScript)