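; Powerup pickup actor that picks one of four random types on spawn: shield, floating, missile bullet or stun bullet.
; It feeds that type's mesh to a Niagara system as the shape to form, then after a short delay sets the matching static mesh and shared pickup material.
; When destroyed, it calls PowerupsTake on the TT_PowerupSpawner_BP actors in the level.
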(event Custom|ChangeMat
  (bind _powerupmesh (Variables|Default|GetpowerupMesh))
  (bind _returnvalue (Class|TTPowerup|GetPowerupType))
  (switch Utilities|FlowControl|Switch|SwitchonEPowerupType _returnvalue
    (:PT_none
      (Development|PrintString "Pickup_BP: PT_None"))
    (:PT_shild
      (Components|StaticMesh|SetStaticMesh _powerupmesh "/Game/Assets/StaticMesh/Pickups/TT_ShieldPowerup_StaticMesh.TT_ShieldPowerup_StaticMesh")
      (Rendering|Material|SetMaterial (Variables|Default|GetpowerupMesh) 0 "/Game/Assets/Materials/AT_Pickup_Material.AT_Pickup_Material" :!label _label))
    (:PT_floating
      ;[1 1 1] Set when ade
      (Components|StaticMesh|SetStaticMesh _powerupmesh "/Game/Assets/StaticMesh/Pickups/Levitation_Chevron.Levitation_Chevron")
      (goto _label))
    (:PT_missileBullet
      ;[1 1 1] Set to skull
      (Components|StaticMesh|SetStaticMesh _powerupmesh "/Game/Assets/StaticMesh/Pickups/TT_SuperMissilePowerup_StaticMesh.TT_SuperMissilePowerup_StaticMesh")
      (goto _label))
    (:PT_stunBullet
      (Components|StaticMesh|SetStaticMesh _powerupmesh "/Game/Assets/StaticMesh/Pickups/TT_StunMissilePowerup_StaticMesh.TT_StunMissilePowerup_StaticMesh")
      (goto _label))))

(event Custom|Spawn%20Anim
  (bind _output_get (Variables|Default|SetpowerupType (Utilities|Select :Index (Math|Random|RandomIntegerinRange 0 3) :Option%200 "PT_shild" :Option%201 "PT_floating" :Option%202 "PT_missileBullet" :Option%203 "PT_stunBullet")))
  (Class|NiagaraFunctionLibrary|OverrideSystemUserVariableStaticMesh (Variables|Default|GetNiagara) "User.MeshToForm" (.Value (Utilities|Map|Find (Variables|Default|GetMeshes) _output_get)))
  (Utilities|FlowControl|Delay 0.2)
  (CallFunction|MakeAvailable))

(event Custom|Make%20Available
  (CallFunction|ChangeMat))

(event EventBeginPlay
  (CallFunction|SpawnAnim))

(event EventDestroyed
  (bind _outactors (Actor|GetAllActorsOfClass "/Game/Blueprints/Powerups/TT_PowerupSpawner_BP.TT_PowerupSpawner_BP_C"))
  (Default|PowerupsTake _outactors))

(fn ConstructionScript)