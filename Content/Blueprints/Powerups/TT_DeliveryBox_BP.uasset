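; Delivery box that drops to the ground and bursts open to deliver a random powerup.
; The construction script traces downward for a landing point, and the Falling timeline lerps the box there, though no event here starts it.
; On finish it spawns TT_Powerup_BP with one of four types, briefly physics-scatters its side pieces, then destroys itself.
; A parallel delayed branch is wired to destroy the powerup later.
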(event EventBeginPlay)

(fn ConstructionScript
  (Variables|Default|SetAll%20Sides (Utilities|Array|MakeArray (Variables|Default|GetSide%201) (Variables|Default|GetSide%202) (Variables|Default|GetSide%203) (Variables|Default|GetSide%204) (Variables|Default|GetSide%206)))
  (bind _output_get (Variables|Default|SetPosition%20before%20fall (Transformation|GetActorLocation)))
  (bind _outhit (Collision|LineTraceByChannel _output_get (- _output_get "0, 0,1000.000000") "TraceTypeQuery1" false 0 "ForOneFrame"))
  (Variables|Default|SetPosition%20of%20landing (+ (.location _outhit) "0, 0,25.000000")))