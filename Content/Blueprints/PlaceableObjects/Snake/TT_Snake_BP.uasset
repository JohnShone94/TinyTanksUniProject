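; TT_Snake_BP is a snake actor whose body slides along a spline path, bending to follow its curve.
; The construction script adds a spline mesh component and stores it as Snake.
; On BeginPlay, the SnakeMove timeline drives a distance from zero to the spline's full length.
; Each update sets the mesh start at that distance and its end a fixed distance behind, using the spline's local positions and tangents.
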(event EventBeginPlay
  (bind _spline (Variables|Default|GetSpline))
  (bind _alpha (Timeline|Snake%20Move PlayFromStart)
    (:Update
      (SplineMesh|SetStartandEnd (Variables|Default|GetSnake) (Spline|GetLocationatDistanceAlongSpline _spline (Math|Float|Lerp 0.0 (Spline|GetSplineLength _spline) _alpha) "Local") (Spline|GetTangentatDistanceAlongSpline _spline (Math|Float|Lerp 0.0 (Spline|GetSplineLength _spline) _alpha) "Local") (Spline|GetLocationatDistanceAlongSpline _spline (- (Math|Float|Lerp 0.0 (Spline|GetSplineLength _spline) _alpha) 3e+02) "Local") (Spline|GetTangentatDistanceAlongSpline _spline (- (Math|Float|Lerp 0.0 (Spline|GetSplineLength _spline) _alpha) 3e+02) "Local") true :!class /Script/Engine.SplineMeshComponent))))

(event Collision|EventActorBeginOverlap
  (params (OtherActor :type Actor%20Object%20Reference)))

(event EventTick
  (params (DeltaSeconds :type Float%20%28single-precision%29)))

(fn ConstructionScript
  (bind _returnvalue (AddComponent|AddSplineMeshComponent false))
  (Transformation|AttachComponentToComponent _returnvalue "None" "KeepRelative" "KeepRelative" "KeepRelative" true)
  (Variables|Default|SetSnake _returnvalue))