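; Spike tile hazard that damages TT_TankBase tanks overlapping its DamageBox while CanDamage is set.
; Entering RiseBox, unless TriggeredByButton is set, starts a delayed timeline that lerps DamageBox up and back, enabling damage only near EndLocation.
; A separate button event drives another raise timeline in world space without updating CanDamage.
; The nodes computing StartLocation and EndLocation from DamageBox are disconnected.
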(event OnComponentBeginOverlap(Damagebox)
  (params (OverlappedComponent :type Primitive%20Component%20Object%20Reference) (OtherActor :type Actor%20Object%20Reference) (OtherComp :type Primitive%20Component%20Object%20Reference) (OtherBodyIndex :type Integer) (bFromSweep :type Boolean) (SweepResult :type Hit%20Result%20Structure%20%28by%20ref%29))
  (bind _astt_tank_base (Utilities|Casting|CastToTT_TankBase OtherActor))
  (if (Variables|Default|GetcanDamage)
    (Class|TTTankBase|DamageTank _astt_tank_base)
    (Utilities|FlowControl|Delay 1.0)))

(event OnComponentBeginOverlap(Risebox)
  (params (OverlappedComponent :type Primitive%20Component%20Object%20Reference) (OtherActor :type Actor%20Object%20Reference) (OtherComp :type Primitive%20Component%20Object%20Reference) (OtherBodyIndex :type Integer) (bFromSweep :type Boolean) (SweepResult :type Hit%20Result%20Structure%20%28by%20ref%29))
  (if (not (Variables|Default|GetTriggered%20by%20button?))
    (Utilities|FlowControl|Delay 1.5)
    (if (not (Variables|Default|GetSpikes%20are%20moving?))
      (Variables|Default|SetSpikes%20are%20moving? true)
      (Utilities|Casting|CastToTT_TankBase OtherActor)
      (CallFunction|RiseandLowerSpikes))))

(event Custom|Rise%20and%20lower%20spikes
  (bind _damage_box (Variables|Default|GetDamage%20box))
  (bind _end_location (Variables|Default|GetEnd%20Location))
  (bind _relativelocation (Variables|/Script/Engine.SceneComponent|GetRelativeLocation _damage_box))
  (bind _returnvalue (Math|Vector|Equal(Vector) _relativelocation _end_location 1.0))
  (bind _move_spikes (Timeline|Rise%20Spikes%20then%20lower PlayFromStart)
    (:Update
      (Transformation|SetRelativeLocation (Variables|Default|GetDamage%20box) (Math|Vector|Lerp(Vector) (Variables|Default|GetStart%20Location) (Variables|Default|GetEnd%20Location) _move_spikes) false false)
      (Development|PrintString (Utilities|String|ToString(Boolean) _returnvalue))
      (if _returnvalue
        (Variables|Default|SetcanDamage true)
        (else
          (Variables|Default|SetcanDamage false))))
    (:Finished
      (Variables|Default|SetSpikes%20are%20moving? false))))

(event Custom|Button%20Pressed]
  (bind _move_spikes (Timeline|Raise%20Spikes PlayFromStart)
    (:Update
      (Transformation|SetWorldLocation (Variables|Default|GetDamage%20box) (Math|Vector|Lerp(Vector) (Variables|Default|GetStart%20Location) (Variables|Default|GetEnd%20Location) _move_spikes) false false))))

(fn ConstructionScript)