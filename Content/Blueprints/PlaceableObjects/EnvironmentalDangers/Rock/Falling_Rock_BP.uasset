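; Falling rock hazard that crushes tanks, triggered by Rockfall or automatically shortly after BeginPlay.
; A timeline-driven decal shadow grows as a warning with camera shake and randomly scaled physics pebbles, then the rock simulates physics and drops.
; First impact shakes the camera and starts a looping cracked-material effect.
; Hits kill tanks until the rock lands on something else; afterwards player contact destroys it, as do magic missiles anytime.
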(event Custom|Rock%20fall
  ;[1 1 1] Spawn Pebbles before falling
  (Utilities|FlowControl|DoOnce false
    (:Completed
      (bind _returnvalue (Rendering|Material|CreateDynamicMaterialInstance (Variables|Default|GetDecal) :!class /Script/Engine.DecalComponent))
      (Variables|Default|SetSet%20scalar%20parameter _returnvalue)
      (CallFunction|ShaddowChange)
      (Rendering|SetVisibility (Variables|Default|GetDecal) true false)
      (Utilities|FlowControl|Delay 2.0)
      (Utilities|FlowControl|Sequence
        (:then_0
          (Utilities|FlowControl|Delay 2.0)
          (Physics|SetSimulatePhysics (Variables|Default|GetRock%202.0) true)
          (Class|PrimitiveComponent|SetPhysicsAngularVelocityinDegrees (Variables|Default|GetRock%202.0) "180.000000,90.000000, 0" false "None"))
        (:then_1
          (bind _returnvalue_2 (AddComponent|AddStaticMeshComponent false (Math|Transform|MakeTransform "0.000000,0.0,-100.000000" "0, 0, 0" (Utilities|Select :Index (Math|Random|RandomInteger 2) :Option%200 "0.010000,0.010000,0.010000" :Option%201 "0.012500,0.012500,0.012500" :Option%202 "0.015000,0.015000,0.015000"))))
          (Rendering|SetCastShadow _returnvalue_2 false)
          (Utilities|FlowControl|Delay (Math|Random|RandomFloatinRange 0.1 0.5))
          (Physics|SetSimulatePhysics _returnvalue_2 true)
          (Class|PrimitiveComponent|SetPhysicsAngularVelocityinDegrees _returnvalue_2 "180.000000,90.000000, 0" false "None")
          (Utilities|Array|Add (Variables|Default|GetList%20of%20Spawned%20rocks) _returnvalue_2)
          (bind _returnvalue_3 (AddComponent|AddStaticMeshComponent false (Math|Transform|MakeTransform "-0.000000,0.0,-50.000000" "0, 0, 0" (Utilities|Select :Index (Math|Random|RandomInteger 2) :Option%200 "0.010000,0.010000,0.010000" :Option%201 "0.012500,0.012500,0.012500" :Option%202 "0.015000,0.015000,0.015000"))))
          (Rendering|SetCastShadow _returnvalue_3 false)
          (Utilities|FlowControl|Delay (Math|Random|RandomFloatinRange 0.1 0.5))
          (Physics|SetSimulatePhysics _returnvalue_3 true)
          (Class|PrimitiveComponent|SetPhysicsAngularVelocityinDegrees _returnvalue_3 "180.000000,-80.000000, 0" false "None")
          (Utilities|Array|Add (Variables|Default|GetList%20of%20Spawned%20rocks) _returnvalue_3)
          (bind _returnvalue_4 (AddComponent|AddStaticMeshComponent false (Math|Transform|MakeTransform "0.000000,0.0,-60.000000" "0, 0, 0" (Utilities|Select :Index (Math|Random|RandomInteger 2) :Option%200 "0.010000,0.010000,0.010000" :Option%201 "0.012500,0.012500,0.012500" :Option%202 "0.015000,0.015000,0.015000"))))
          (Rendering|SetCastShadow _returnvalue_4 false)
          (Utilities|FlowControl|Delay (Math|Random|RandomFloatinRange 0.1 0.5))
          (Physics|SetSimulatePhysics _returnvalue_4 true)
          (Class|PrimitiveComponent|SetPhysicsAngularVelocityinDegrees _returnvalue_4 "180.000000,90.000000, 0" false "None")
          (Utilities|Array|Add (Variables|Default|GetList%20of%20Spawned%20rocks) _returnvalue_4))))))

(event Custom|Rock%20destroyed
  ;[1 1 1] Destroy actor sequence
  (Actor|DestroyActor))

(event Custom|Shaddow%20change
  ;[1 1 1] Shaddow Control
  (Camera|PlayWorldCameraShake "/Game/Blueprints/Camera/Pre_rockfall_CAmShake.Pre_rockfall_CAmShake_C" "0, 0, 0" 0.0 1e+05)
  (bind (_direction _shaddow_intensity _shaddow_size) (Timeline|Shaddown%20gets%20closer PlayFromStart)
    (:Update
      (Transformation|SetWorldScale3D (Variables|Default|GetDecal) (Math|Vector|MakeVector 1.0 _shaddow_size _shaddow_size))
      (Rendering|Material|SetScalarParameterValue (Variables|Default|GetSet%20scalar%20parameter) "Shaddow intensity" _shaddow_intensity :!class /Script/Engine.MaterialInstanceDynamic))))

(event Custom|Clear%20Rocks)

(event Custom|CustomEvent_0)

(event Collision|EventHit
  (params (MyComp :type Primitive%20Component%20Object%20Reference) (Other :type Actor%20Object%20Reference) (OtherComp :type Primitive%20Component%20Object%20Reference) (bSelfMoved :type Boolean) (HitLocation :type Vector :default "0, 0, 0") (HitNormal :type Vector :default "0, 0, 0") (NormalImpulse :type Vector :default "0, 0, 0") (Hit :type Hit%20Result%20Structure%20%28by%20ref%29))
  (bind _rock_2_0 (Variables|Default|GetRock%202.0))
  (bind _rock_2_0_2 (Variables|Default|GetRock%202.0))
  ;[1 1 1] When rock lands
  (Utilities|FlowControl|Sequence
    (:then_0
      (Utilities|FlowControl|DoOnce false
        (:Completed
          (Camera|PlayWorldCameraShake "/Game/Blueprints/Camera/RockFall_CamShake.RockFall_CamShake_C" "0, 0, 0" 1.0 1e+05 0.0)
          (Rendering|Material|SetMaterial (Variables|Default|GetRock%202.0) 0 "/Game/Assets/Materials/TT_CrackedTIle.TT_CrackedTIle")
          (bind _newtrack_0 (Timeline|Timeline_0 Play)
            (:Update
              (Rendering|Material|SetScalarParameterValueonMaterials (Variables|Default|GetRock%202.0) "None" _newtrack_0))
            (:Finished
              (if true
                (Timeline|Timeline_0 PlayFromStart)))))))
    (:then_1
      (if (Variables|Default|Getshould%20rock%20kill%20tank)
        (Utilities|FlowControl|Sequence
          (:then_0
            (bind _astt_tank_base (Utilities|Casting|CastToTT_TankBase Other)
              (:then
                (Class|TTTankBase|KillTank _astt_tank_base true)
                (Physics|SetEnableGravity _rock_2_0_2 false)
                (Physics|SetPhysicsLinearVelocity _rock_2_0_2 "0, 0, 0" false "None")
                (Physics|SetSimulatePhysics _rock_2_0_2 false)
                (Variables|Default|SetCan%20rock%20be%20destroyed true)
                (Utilities|FlowControl|DoOnce false
                  (:Completed
                    (for _array_element (Variables|Default|GetList%20of%20Spawned%20rocks)
                      (Components|DestroyComponent _array_element)))))
              (:CastFailed
                (Variables|Default|Setshould%20rock%20kill%20tank false)
                (Physics|SetSimulatePhysics (Variables|Default|GetRock%202.0) false)
                (Class|PrimitiveComponent|SetAllPhysicsLinearVelocity _rock_2_0 "0, 0, 0" false)
                (Class|PrimitiveComponent|SetAllPhysicsAngularVelocityinDegrees _rock_2_0 (Math|Vector|MakeVector 0.0 0.0 0.0) false))))
          (:then_1
            (bind _astt_player_bp (Utilities|Casting|CastToTT_Player_BP Other))
            (Utilities|FlowControl|DoOnce false
              (:Completed
                (Default|TankBlowsUp _astt_player_bp)))))
        (else
          (Utilities|Casting|CastToTT_Player_BP Other)
          (Actor|DestroyActor))))
    (:then_2
      (bind _astt_magic_missile (Utilities|Casting|CastToTT_MagicMissile Other))
      (Actor|DestroyActor)
      (Actor|DestroyActor _astt_magic_missile))))

(event EventBeginPlay
  ;[1 1 1] On spawn
  (Utilities|FlowControl|Delay 3.0)
  ;[1 1 1] Spawn Pebbles before falling
  (Utilities|FlowControl|DoOnce false
    (:Completed
      (bind _returnvalue (Rendering|Material|CreateDynamicMaterialInstance (Variables|Default|GetDecal) :!class /Script/Engine.DecalComponent))
      (Variables|Default|SetSet%20scalar%20parameter _returnvalue)
      (CallFunction|ShaddowChange)
      (Rendering|SetVisibility (Variables|Default|GetDecal) true false)
      (Utilities|FlowControl|Delay 2.0)
      (Utilities|FlowControl|Sequence
        (:then_0
          (Utilities|FlowControl|Delay 2.0)
          (Physics|SetSimulatePhysics (Variables|Default|GetRock%202.0) true)
          (Class|PrimitiveComponent|SetPhysicsAngularVelocityinDegrees (Variables|Default|GetRock%202.0) "180.000000,90.000000, 0" false "None"))
        (:then_1
          (bind _returnvalue_2 (AddComponent|AddStaticMeshComponent false (Math|Transform|MakeTransform "0.000000,0.0,-100.000000" "0, 0, 0" (Utilities|Select :Index (Math|Random|RandomInteger 2) :Option%200 "0.010000,0.010000,0.010000" :Option%201 "0.012500,0.012500,0.012500" :Option%202 "0.015000,0.015000,0.015000"))))
          (Rendering|SetCastShadow _returnvalue_2 false)
          (Utilities|FlowControl|Delay (Math|Random|RandomFloatinRange 0.1 0.5))
          (Physics|SetSimulatePhysics _returnvalue_2 true)
          (Class|PrimitiveComponent|SetPhysicsAngularVelocityinDegrees _returnvalue_2 "180.000000,90.000000, 0" false "None")
          (Utilities|Array|Add (Variables|Default|GetList%20of%20Spawned%20rocks) _returnvalue_2)
          (bind _returnvalue_3 (AddComponent|AddStaticMeshComponent false (Math|Transform|MakeTransform "-0.000000,0.0,-50.000000" "0, 0, 0" (Utilities|Select :Index (Math|Random|RandomInteger 2) :Option%200 "0.010000,0.010000,0.010000" :Option%201 "0.012500,0.012500,0.012500" :Option%202 "0.015000,0.015000,0.015000"))))
          (Rendering|SetCastShadow _returnvalue_3 false)
          (Utilities|FlowControl|Delay (Math|Random|RandomFloatinRange 0.1 0.5))
          (Physics|SetSimulatePhysics _returnvalue_3 true)
          (Class|PrimitiveComponent|SetPhysicsAngularVelocityinDegrees _returnvalue_3 "180.000000,-80.000000, 0" false "None")
          (Utilities|Array|Add (Variables|Default|GetList%20of%20Spawned%20rocks) _returnvalue_3)
          (bind _returnvalue_4 (AddComponent|AddStaticMeshComponent false (Math|Transform|MakeTransform "0.000000,0.0,-60.000000" "0, 0, 0" (Utilities|Select :Index (Math|Random|RandomInteger 2) :Option%200 "0.010000,0.010000,0.010000" :Option%201 "0.012500,0.012500,0.012500" :Option%202 "0.015000,0.015000,0.015000"))))
          (Rendering|SetCastShadow _returnvalue_4 false)
          (Utilities|FlowControl|Delay (Math|Random|RandomFloatinRange 0.1 0.5))
          (Physics|SetSimulatePhysics _returnvalue_4 true)
          (Class|PrimitiveComponent|SetPhysicsAngularVelocityinDegrees _returnvalue_4 "180.000000,90.000000, 0" false "None")
          (Utilities|Array|Add (Variables|Default|GetList%20of%20Spawned%20rocks) _returnvalue_4))))))

(fn ConstructionScript)