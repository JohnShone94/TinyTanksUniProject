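; Rock spawner hazard that drops falling rocks onto empty cells of the world grid.
; Each SpawnRock call rolls between LowRange and MaxRange, and each miss raises LowRange up to a cap, narrowing the roll until ResetLevel zeroes it.
; A hit picks a random empty cell on every TT_WorldGrid, marks it filled and spawns a Falling_Rock_BP above it with that cell as landing position.
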(event Custom|SpawnRock
  (if (== 5 (Math|Random|RandomIntegerinRange (Variables|Default|GetLowRange) (Variables|Default|GetMaxRange)))
    ;[0 1 0.0615] Spawn
    (bind _outactors (Actor|GetAllActorsOfClass "/Script/TinyTanksUniProject.TT_WorldGrid"))
    (for _array_element _outactors
      (bind _returnvalue (Class|TTWorldGrid|GetRandomEmptyCell _array_element))
      (Utilities|IsValid _returnvalue
        (:Is%20Valid
          (Class|TTGridCell|SetCellFilled _returnvalue true)
          (bind _returnvalue_2 (Game|SpawnActorfromClass "/Game/Blueprints/PlaceableObjects/EnvironmentalDangers/Rock/Falling_Rock_BP.Falling_Rock_BP_C" (Math|Transform|MakeTransform (+ (Transformation|GetActorLocation _returnvalue) "0,0,750.000000") "0, 0, 0" "1,1,1") "Undefined" 0 0))
          (Variables|/Game/Blueprints/PlaceableObjects/EnvironmentalDangers/Rock/Falling_Rock_BP.Falling_Rock_BP_C|SetLandingPosition _returnvalue_2 (+ (Transformation|GetActorLocation _returnvalue) "0,0,30.000000")))))
    (else
      ;[1 0 0] Fail
      (if (not (== (Variables|Default|GetLowRange) 5))
        (Variables|Default|SetLowRange (+ (Variables|Default|GetLowRange) 1))))))

(event Custom|ResetLevel
  (Variables|Default|SetLowRange 0))

(fn ConstructionScript)