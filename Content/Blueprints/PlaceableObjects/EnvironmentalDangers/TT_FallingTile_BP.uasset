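; Environmental hazard tile that drops away shortly after a tank enters its trigger box, then returns to its original spot.
; After a random delay, the collision component simulates physics with a random angular impulse to make it tumble.
; Physics then switches off, and after a pause a timeline lerps the tile back to its starting transform and re-arms it.
; An older counter-based fall-and-destroy chain remains in the graph, disconnected from the overlap logic.
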(event OnComponentBeginOverlap(Box)
  (params (OverlappedComponent :type Primitive%20Component%20Object%20Reference) (OtherActor :type Actor%20Object%20Reference) (OtherComp :type Primitive%20Component%20Object%20Reference) (OtherBodyIndex :type Integer) (bFromSweep :type Boolean) (SweepResult :type Hit%20Result%20Structure%20%28by%20ref%29))
  (bind _colision (Variables|Default|GetColision))
  (bind _colision_2 (Variables|Default|GetColision))
  (Utilities|Casting|CastToTT_TankBase OtherActor)
  (if (not (Variables|Default|GetIs%20falling))
    (Variables|Default|SetIs%20falling true)
    (Utilities|FlowControl|Delay (Math|Random|RandomFloatinRange 0.5 1.25))
    (Physics|SetSimulatePhysics _colision_2 true)
    (Physics|SetEnableGravity _colision_2 true)
    (Class|PrimitiveComponent|AddAngularImpulseinDegrees (Variables|Default|GetColision) (+ (Utilities|Select :Index (Math|Random|RandomIntegerinRange 0 2) :Option%200 "300.000000, 0, 0" :Option%201 "0,300.000000, 0" :Option%202 "0, 0,300.000000") (Utilities|Select :Index (Math|Random|RandomIntegerinRange 0 2) :Option%200 "300.000000, 0, 0" :Option%201 "0,300.000000, 0" :Option%202 "0, 0,300.000000")) "None" false)
    (Utilities|FlowControl|Delay 2.0)
    (Variables|Default|SetFallen%20Location (Transformation|GetWorldTransform (Variables|Default|GetColision)))
    (Physics|SetEnableGravity _colision false)
    (Physics|SetSimulatePhysics _colision false)
    (Utilities|FlowControl|Delay 3.0)
    (bind _move (Timeline|Move%20back%20to%20spot PlayFromStart)
      (:Update
        (Transformation|SetWorldTransform (Variables|Default|GetColision) (Math|Transform|Lerp(Transform) (Variables|Default|GetFallen%20Location) (Variables|Default|GetOrigin%20Location) _move) false true))
      (:Finished
        (Variables|Default|SetIs%20falling false)))))

(event OnComponentEndOverlap(Box)
  (params (OverlappedComponent :type Primitive%20Component%20Object%20Reference) (OtherActor :type Actor%20Object%20Reference) (OtherComp :type Primitive%20Component%20Object%20Reference) (OtherBodyIndex :type Integer))
  (if (not (Variables|Default|GetIs%20falling))
    (Utilities|Casting|CastToTT_TankBase OtherActor)))

(event Custom|Fall
  (bind _colision (Variables|Default|GetColision))
  ;[1 1 1] Old SHit
  (bind _counter (Utilities|FlowControl|DoN 4 :!label _label)
    (:Exit
      (if (== _counter 4)
        (Variables|Default|SetIs%20falling true)
        (Physics|SetSimulatePhysics _colision true)
        (Physics|SetEnableGravity _colision true)
        (Utilities|FlowControl|Delay 0.5)
        (Utilities|FlowControl|Delay 3.0)
        (Actor|DestroyActor)
        (else
          (Utilities|FlowControl|Delay 0.75)
          (if (Variables|Default|GetShould%20Fall?)
            (goto _label)
            (else
              (CallFunction|StopFall))))))))

(event Custom|Reset%20fall
  (bind _colision (Variables|Default|GetColision))
  ;[1 1 1] Old SHit
  (Utilities|FlowControl|Sequence
    (:then_0
      (Utilities|FlowControl|DoOnce false) ; enters at Reset
    )
    (:then_1
      (Utilities|FlowControl|DoN 4) ; enters at Reset
    )))

(event Custom|Stop%20fall
  ;[1 1 1] Old SHit
  (CallFunction|ResetFall))

(event EventBeginPlay
  (Variables|Default|SetOrigin%20Location (Transformation|GetWorldTransform (Variables|Default|GetColision))))

(fn ConstructionScript)