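; TT_DestructableWall_BP is a wall that destroys itself when hit by a TT_MagicMissile.
; The hit optionally plays a rockfall camera shake, then tells the first TT_RockSpawnerBP found in the level to spawn a rock.
; A looping Throb timeline writes to a material scalar on the Cube, though its parameter name is None.
; The construction script gives the Cube a random quarter-turn rotation.
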(event EventBeginPlay
  (bind _newtrack_0 (Timeline|Throb PlayFromStart)
    (:Update
      (Rendering|Material|SetScalarParameterValueonMaterials (Variables|Default|GetCube) "None" _newtrack_0))
    (:Finished
      (if true
        (Timeline|Throb PlayFromStart)))))

(event Collision|EventHit
  (params (MyComp :type Primitive%20Component%20Object%20Reference) (Other :type Actor%20Object%20Reference) (OtherComp :type Primitive%20Component%20Object%20Reference) (bSelfMoved :type Boolean) (HitLocation :type Vector :default "0, 0, 0") (HitNormal :type Vector :default "0, 0, 0") (NormalImpulse :type Vector :default "0, 0, 0") (Hit :type Hit%20Result%20Structure%20%28by%20ref%29))
  (Utilities|Casting|CastToTT_MagicMissile Other)
  (if (Variables|Default|GetShould%20casue%20rumble?)
    (Camera|PlayWorldCameraShake "/Game/Blueprints/Camera/Pre_rockfall_CAmShake.Pre_rockfall_CAmShake_C" "0, 0, 0" 1e+01 1e+05))
  (Utilities|FlowControl|Sequence
    (:then_0
      (bind _outactors (Actor|GetAllActorsOfClass "/Game/Blueprints/PlaceableObjects/EnvironmentalDangers/Rock/TT_RockSpawnerBP.TT_RockSpawnerBP_C"))
      (Default|SpawnRock (Utilities|Array|Get(acopy) _outactors)))
    (:then_1
      (Actor|DestroyActor))))

(fn ConstructionScript
  (Transformation|SetRelativeRotation (Variables|Default|GetCube) (Utilities|Select :Index (Math|Random|RandomIntegerinRange 0 3) :Option%200 "0,90.000000,0.000000" :Option%201 "0.000000,180.000000,0.000000" :Option%202 "0.000000,270.000000,0.000000" :Option%203 "0, 0, 0") false false))