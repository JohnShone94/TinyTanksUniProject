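; Placeable vine actor that builds a vine along an editable spline in its construction script; the event graph is empty.
; It adds one spline mesh per mesh length, each a random pick from a mesh array with the vine material, fitted using length-clamped tangents.
; An optional Leaves pass, flagged as a performance cutoff, randomly adds leaf static meshes at roughly 30% of segment starts.
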(event EventBeginPlay)

(event Collision|EventActorBeginOverlap
  (params (OtherActor :type Actor%20Object%20Reference)))

(event EventTick
  (params (DeltaSeconds :type Float%20%28single-precision%29)))

(fn ConstructionScript
  (bind _spline (Variables|Default|GetSpline))
  (bind _arrayofpossiblemeshes (Variables|Default|GetArrayOfPossibleMeshes))
  (Variables|Default|SetArrayOfMeshes (Utilities|Array|MakeArray 0))
  (LocalVariables|SetLength (* (.x (Transformation|GetActorScale3D)) (Variables|Default|GetMeshLength)))
  (for _index (range 0 (Math|Float|Truncate (/ (Spline|GetSplineLength (Variables|Default|GetSpline)) (Variables|Default|GetMeshLength)))) ; Loop for every mesh needed
    (bind _returnvalue (AddComponent|AddSplineMeshComponent false))
    (Rendering|Material|SetMaterial _returnvalue 0 "/Game/Assets/Materials/TT_Vine_Material.TT_Vine_Material")
    (Components|StaticMesh|SetStaticMesh _returnvalue (Utilities|Array|Get(acopy) _arrayofpossiblemeshes (Math|Random|RandomIntegerinRange 0 (- (Utilities|Array|Length _arrayofpossiblemeshes) 1))))
    (SplineMesh|SetForwardAxis _returnvalue "X" true)
    (Utilities|Array|Add (Variables|Default|GetArrayOfMeshes) _returnvalue)
    (SplineMesh|SetStartandEnd _returnvalue (Spline|GetLocationatDistanceAlongSpline _spline (* _index (Variables|Default|GetMeshLength)) "Local") (Math|Vector|ClampVectorSize (Spline|GetTangentatDistanceAlongSpline _spline (* _index (Variables|Default|GetMeshLength)) "Local") 0.0 (Variables|Default|GetMeshLength)) (Spline|GetLocationatDistanceAlongSpline _spline (* (+ _index 1) (Variables|Default|GetMeshLength)) "Local") (Math|Vector|ClampVectorSize (Spline|GetTangentatDistanceAlongSpline _spline (* (+ _index 1) (Variables|Default|GetMeshLength)) "Local") 0.0 (Variables|Default|GetMeshLength)) true :!class /Script/Engine.SplineMeshComponent))
  ;[1 1 1] CUT OFF FOR PERFORMANCE!!!
  (if (Variables|Default|GetLeaves)
    (for _array_element (Variables|Default|GetArrayOfMeshes)
      (if (> (Math|Random|RandomFloat) 0.7)
        (bind _returnvalue_2 (AddComponent|AddStaticMeshComponent false (Math|Transform|MakeTransform (SplineMesh|GetStartPosition _array_element) "0, 0, 0" "1,1,1")))
        (Components|StaticMesh|SetStaticMesh _returnvalue_2 "/Game/Assets/StaticMesh/Foliage/TT_VineLeaf_StaticMesh.TT_VineLeaf_StaticMesh")))))