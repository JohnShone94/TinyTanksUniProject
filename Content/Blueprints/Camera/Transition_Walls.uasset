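; Level transition wall actor: two sliding doors and a large wheel that open and close with camera shakes.
; On BeginPlay, after a delay, timelines drop the wheel and animate its text glow, then slide the doors apart as the wheel rolls away.
; Close slides the doors shut and calls LevelTransitionP1 on TT_MainCam_BP actors.
; Open, also triggered by Changescore, replays the opening motion and calls LevelTransitionP2 when finished.
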(event Custom|Open%20first%20time
  (Variables|Default|SetWheel%20Current (Transformation|GetWorldLocation (Variables|Default|GetBeeg%20Wheel)))
  (Variables|Default|SetRight%20current (Transformation|GetWorldLocation (Variables|Default|GetRight)))
  (Variables|Default|SetLEft%20Current (Transformation|GetWorldLocation (Variables|Default|GetLeft)))
  (Utilities|FlowControl|Sequence
    (:then_0
      (Camera|PlayWorldCameraShake "/Game/Blueprints/Camera/Doors_open_Shake.Doors_open_Shake_C" "0, 0, 0" 1.0 1e+05 0.0))
    (:then_1
      (bind _open_dat_derr_door (Timeline|oPEN%20dEM%20DOORS PlayFromStart)
        (:Update
          (Utilities|FlowControl|Sequence
            (:then_0
              (Transformation|SetWorldLocation (Variables|Default|GetRight) (Math|Vector|Lerp(Vector) (Variables|Default|GetRight%20current) (+ (Variables|Default|GetRight%20current) "250.000000, 0, 0") _open_dat_derr_door) false false))
            (:then_1
              (Transformation|SetWorldLocation (Variables|Default|GetLeft) (Math|Vector|Lerp(Vector) (Variables|Default|GetLEft%20Current) (- (Variables|Default|GetLEft%20Current) "250.000000, 0, 0") _open_dat_derr_door) false false))
            (:then_2
              (Transformation|SetWorldLocation (Variables|Default|GetBeeg%20Wheel) (Math|Vector|Lerp(Vector) (Variables|Default|GetWheel%20Current) (- (Variables|Default|GetWheel%20Current) "250.000000, 0, 0") _open_dat_derr_door) false false))
            (:then_3
              (Transformation|AddRelativeRotation (Variables|Default|GetBeeg%20Wheel) "0.650000, 0, 0" false false))))))))

(event Custom|Setup
  (Utilities|FlowControl|Delay 3.0)
  (bind _open_dat_derr_door (Timeline|Drop%20Da%20Dial PlayFromStart)
    (:Update
      (Transformation|SetRelativeLocation (Variables|Default|GetBeeg%20Wheel) (Math|Vector|Lerp(Vector) "0.000000,150.000000, 0" "0,60.000000, 0" _open_dat_derr_door) false false))
    (:Finished
      (Camera|PlayWorldCameraShake "/Game/Blueprints/Camera/Explosion_CamShake.Explosion_CamShake_C" "0.000000, 0, 0" 1.0 1e+05 0.0)
      (bind _open_dat_derr_door_2 (Timeline|Timeline_0 PlayFromStart)
        (:Update
          (Rendering|Material|SetScalarParameterValueonMaterials (Variables|Default|GetBeeg%20Wheel) "Text glow" _open_dat_derr_door_2))
        (:Finished
          (CallFunction|OpenFirstTime))))))

(event Custom|Close
  (Variables|Default|SetRight%20current (Transformation|GetWorldLocation (Variables|Default|GetRight)))
  (Variables|Default|SetLEft%20Current (Transformation|GetWorldLocation (Variables|Default|GetLeft)))
  (bind _open_dat_derr_door (Timeline|Close%20dem%20Doors PlayFromStart)
    (:Update
      (Utilities|FlowControl|Sequence
        (:then_0
          (Transformation|SetWorldLocation (Variables|Default|GetLeft) (Math|Vector|Lerp(Vector) (Variables|Default|GetLEft%20Current) (+ (Variables|Default|GetLEft%20Current) "250.000000, 0, 0") _open_dat_derr_door) false false))
        (:then_1
          (Transformation|SetWorldLocation (Variables|Default|GetRight) (Math|Vector|Lerp(Vector) (Variables|Default|GetRight%20current) (- (Variables|Default|GetRight%20current) "250.000000, 0, 0") _open_dat_derr_door) false false))))
    (:Finished
      (Camera|PlayWorldCameraShake "/Game/Blueprints/Camera/Explosion_CamShake.Explosion_CamShake_C" "0, 0, 0" 1.0 1e+05 0.0)
      (bind _outactors (Actor|GetAllActorsOfClass "/Game/Blueprints/Camera/TT_MainCam_BP.TT_MainCam_BP_C"))
      (for _array_element _outactors
        (Default|LevelTransitionP1 _array_element)))))

(event Custom|Open
  (bind _wheel_current (Variables|Default|GetWheel%20Current))
  (Variables|Default|SetRight%20current (Transformation|GetWorldLocation (Variables|Default|GetRight)))
  (Variables|Default|SetLEft%20Current (Transformation|GetWorldLocation (Variables|Default|GetLeft)))
  (Utilities|FlowControl|Sequence
    (:then_0
      (Camera|PlayWorldCameraShake "/Game/Blueprints/Camera/Doors_open_Shake.Doors_open_Shake_C" "0, 0, 0" 1.0 1e+05 0.0))
    (:then_1
      (bind _open_dat_derr_door (Timeline|Timeline_1 PlayFromStart)
        (:Update
          (Utilities|FlowControl|Sequence
            (:then_0
              (Transformation|SetWorldLocation (Variables|Default|GetRight) (Math|Vector|Lerp(Vector) (Variables|Default|GetRight%20current) (+ (Variables|Default|GetRight%20current) "250.000000, 0, 0") _open_dat_derr_door) false false))
            (:then_1
              (Transformation|SetWorldLocation (Variables|Default|GetLeft) (Math|Vector|Lerp(Vector) (Variables|Default|GetLEft%20Current) (- (Variables|Default|GetLEft%20Current) "250.000000, 0, 0") _open_dat_derr_door) false false))
            (:then_2
              (Transformation|SetWorldLocation (Variables|Default|GetBeeg%20Wheel) (Math|Vector|Lerp(Vector) _wheel_current (- _wheel_current "250.000000, 0, 0") _open_dat_derr_door) false false))
            (:then_3
              (Transformation|AddRelativeRotation (Variables|Default|GetBeeg%20Wheel) "0.650000, 0, 0" false false))))
        (:Finished
          (bind _outactors (Actor|GetAllActorsOfClass "/Game/Blueprints/Camera/TT_MainCam_BP.TT_MainCam_BP_C"))
          (for _array_element _outactors
            (Default|LevelTransitionP2 _array_element)))))))

(event Custom|Change%20score
  (CallFunction|Open))

(event EventBeginPlay
  (CallFunction|Setup))

(event Collision|EventActorBeginOverlap
  (params (OtherActor :type Actor%20Object%20Reference)))

(event EventTick
  (params (DeltaSeconds :type Float%20%28single-precision%29)))

(fn ConstructionScript)