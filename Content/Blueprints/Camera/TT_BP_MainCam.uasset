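; Main camera actor for Tiny Tanks that shows the main menu and drives the transitions into gameplay and between streamed levels.
; Setting the game view streams in a level, has the game mode spawn tanks and controllers, then timeline-lerps position, rotation and FOV from menu to game view.
; When the last player stands, it moves out, resets players, cycles to the next streamed level, teleports, and moves back in.
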(event Custom|Change%20level
  (bind _astt_tiny_tanks_game_mode (Utilities|Casting|CastToTT_TinyTanksGameMode (Game|GetGameMode)))
  (Class|TTTinyTanksGameMode|SetCanPlayersControlTanks _astt_tiny_tanks_game_mode true)
  (bind _change_location (Timeline|Transition%20levels PlayFromStart)
    (:Update
      (Transformation|SetActorTransform (Math|Transform|MakeTransform (Math|Vector|Lerp(Vector) (Variables|Default|GetGame_view_Position) (Variables|Default|GetTransition_Position_Pre_TP) _change_location) (Math|Rotator|Lerp(Rotator) (Variables|Default|GetGame_Rotation) (Variables|Default|GetTransition_Rotation) _change_location) "1,1,1")))
    (:Finished
      (Class|TTTinyTanksGameMode|ResetPlayers (Variables|Default|GetGameMode))
      (Game|UnloadStreamLevel(byName) (Utilities|Array|Get(acopy) (Variables|Default|GetStreaming_Levels) (Variables|Default|GetCurrent_Streamed_Levels)) false)
      (if (== (Variables|Default|GetCurrent_Streamed_Levels) (- (Utilities|Array|Length (Variables|Default|GetStreaming_Levels)) 1))
        (Variables|Default|SetCurrent_Streamed_Levels 0)
        (else
          (Variables|Default|SetCurrent_Streamed_Levels (+ (Variables|Default|GetCurrent_Streamed_Levels) 1))))
      (Game|LoadStreamLevel(byName) (Utilities|Array|Get(acopy) (Variables|Default|GetStreaming_Levels) (Variables|Default|GetCurrent_Streamed_Levels)) true)
      (Class|TTTinyTanksGameMode|SpawnPlayerTanks (Variables|Default|GetGameMode))
      (Transformation|SetActorLocation (Variables|Default|GetTransition_Position_Post_TP) false false)
      (bind _change_location_2 (Timeline|Timeline_2 PlayFromStart)
        (:Update
          (Transformation|SetActorTransform (Math|Transform|MakeTransform (Math|Vector|Lerp(Vector) (Variables|Default|GetTransition_Position_Post_TP) (Variables|Default|GetGame_view_Position) _change_location_2) (Math|Rotator|Lerp(Rotator) (Variables|Default|GetTransition_Rotation) (Variables|Default|GetGame_Rotation) _change_location_2) "1,1,1")))
        (:Finished
          (bind _astt_tiny_tanks_game_mode_2 (Utilities|Casting|CastToTT_TinyTanksGameMode (Game|GetGameMode)))
          (Class|TTTinyTanksGameMode|SetCanPlayersControlTanks _astt_tiny_tanks_game_mode_2 true)
          (Class|TTTinyTanksGameMode|SetupPlayerControllers (Variables|Default|GetGameMode) true))))))

(event Custom|Set%20view%20to%20game%20view
  (bind _astt_tiny_tanks_game_mode (Utilities|Casting|CastToTT_TinyTanksGameMode (Game|GetGameMode)))
  (Variables|Default|SetGameMode _astt_tiny_tanks_game_mode)
  (Game|LoadStreamLevel(byName) (Utilities|Array|Get(acopy) (Variables|Default|GetStreaming_Levels) (Variables|Default|GetCurrent_Streamed_Levels)) true)
  (Class|TTTinyTanksGameMode|SpawnPlayerTanks (Variables|Default|GetGameMode))
  (Class|TTTinyTanksGameMode|SpawnPlayerControllers (Variables|Default|GetGameMode))
  (bind (_direction _change_location _newtrack_0) (Timeline|Move%20to%20Main%20view PlayFromStart)
    (:Update
      (Transformation|SetActorLocationAndRotation (Math|Vector|Lerp(Vector) (Variables|Default|GetMenu_View_Position) (Variables|Default|GetGame_view_Position) _change_location) (Math|Rotator|Lerp(Rotator) (Variables|Default|GetMenu_Rotation) (Variables|Default|GetGame_Rotation) _change_location true))
      (Camera|SetFieldOfView (Variables|Default|GetCameraComponent) _newtrack_0))
    (:Finished
      (Class|TTTinyTanksGameMode|SetCanPlayersControlTanks (Variables|Default|GetGameMode) true)
      (Class|TTTinyTanksGameMode|SetupPlayerControllers (Variables|Default|GetGameMode) true))))

(event EventBeginPlay
  (bind _returnvalue (UserInterface|CreateWidget "/Game/Ui/Main_Menu.Main_Menu_C"))
  (UserInterface|Viewport|AddtoViewport _returnvalue 0))

(event EventLastManIsStanding
  (CallFunction|ChangeLevel))

(fn ConstructionScript)