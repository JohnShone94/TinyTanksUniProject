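; Main camera actor for Tiny Tanks that also drives game startup and round-to-round arena changes.
; BeginPlay shows the main menu, loads a streamed level and spawns tanks and controllers through the game mode.
; When the last player stands, Transition_Walls close; a two-phase transition clears pickups and rocks, cycles StreamingLevels, respawns tanks, reopens walls, then restores possession and powerup spawning.
; The menu-to-game camera move timeline is disconnected.
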(event Custom|Change%20level
  (bind _outactors (Actor|GetAllActorsOfClass "/Game/Blueprints/Camera/Transition_Walls.Transition_Walls_C"))
  (for _array_element _outactors
    (Default|Close _array_element)))

(event Custom|Set%20view%20to%20game%20view
  (bind _gamemode (Variables|Default|GetGameMode))
  (bind _outactors (Actor|GetAllActorsOfClass "/Game/Blueprints/Camera/Transition_Walls.Transition_Walls_C"))
  (for _array_element _outactors
    (Default|OpenFirstTime _array_element))
  (Timeline|Open%20Walls PlayFromStart
    (:Update
      (Class|TTTinyTanksGameMode|PlayerPossessTank _gamemode)
      (Class|TTTinyTanksGameMode|SetCanPlayersControlTanks _gamemode true))))

(event Custom|Level%20Transition%20P1
  (if (not (Variables|Default|GetTransitioning))
    (Variables|Default|SetTransitioning true)
    (bind _outactors (Actor|GetAllActorsOfClass "/Game/Blueprints/Powerups/TT_Powerup_BP.TT_Powerup_BP_C"))
    (for _array_element _outactors
      (Actor|DestroyActor _array_element))
    (bind _outactors_2 (Actor|GetAllActorsOfClass "/Game/Blueprints/Players/TT_ShieldDrop_BP.TT_ShieldDrop_BP_C"))
    (for _array_element_2 _outactors_2
      (Actor|DestroyActor _array_element_2))
    (bind _outactors_3 (Actor|GetAllActorsOfClass "/Game/Blueprints/PlaceableObjects/EnvironmentalDangers/Rock/Falling_Rock_BP.Falling_Rock_BP_C"))
    (for _array_element_3 _outactors_3
      (Actor|DestroyActor _array_element_3))
    (bind _outactors_4 (Actor|GetAllActorsOfClass "/Game/Blueprints/Powerups/TT_PowerupSpawner_BP.TT_PowerupSpawner_BP_C"))
    (for _array_element_4 _outactors_4
      (Variables|/Game/Blueprints/Powerups/TT_PowerupSpawner_BP.TT_PowerupSpawner_BP_C|SetShould%20Spawn? _array_element_4 false))
    (Utilities|FlowControl|Delay 1.0)
    (Class|TTTinyTanksGameMode|SetCanPlayersControlTanks (Variables|Default|GetGameMode) true)
    (Class|TTTinyTanksGameMode|ResetPlayers (Variables|Default|GetGameMode))
    (Game|UnloadStreamLevel(byName) (Utilities|Array|Get(acopy) (Variables|Default|GetStreaming_Levels) (Variables|Default|GetCurrent_Streamed_Levels)) false)
    (if (== (Variables|Default|GetCurrent_Streamed_Levels) (- (Utilities|Array|Length (Variables|Default|GetStreaming_Levels)) 1))
      (Variables|Default|SetCurrent_Streamed_Levels 0)
      (else
        (Variables|Default|SetCurrent_Streamed_Levels (+ (Variables|Default|GetCurrent_Streamed_Levels) 1))))
    (Game|LoadStreamLevel(byName) (Utilities|Array|Get(acopy) (Variables|Default|GetStreaming_Levels) (Variables|Default|GetCurrent_Streamed_Levels)) true)
    (Class|TTTinyTanksGameMode|SpawnPlayerTanks (Variables|Default|GetGameMode))
    (bind _outactors_5 (Actor|GetAllActorsOfClass "/Game/Blueprints/Camera/Transition_Walls.Transition_Walls_C"))
    (for _array_element_5 _outactors_5
      (Default|Open _array_element_5))))

(event Custom|Level%20Transition%20P2
  (bind _gamemode (Variables|Default|GetGameMode))
  (Class|TTTinyTanksGameMode|PlayerPossessTank _gamemode)
  (Class|TTTinyTanksGameMode|SetCanPlayersControlTanks _gamemode true)
  (bind _outactors (Actor|GetAllActorsOfClass "/Game/Blueprints/Powerups/TT_PowerupSpawner_BP.TT_PowerupSpawner_BP_C"))
  (for _array_element _outactors
    (Variables|/Game/Blueprints/Powerups/TT_PowerupSpawner_BP.TT_PowerupSpawner_BP_C|SetShould%20Spawn? _array_element true))
  (Variables|Default|SetTransitioning false))

(event EventBeginPlay
  (bind _astt_tiny_tanks_game_mode (Utilities|Casting|CastToTT_TinyTanksGameMode (Game|GetGameMode)))
  (Variables|Default|SetGameMode _astt_tiny_tanks_game_mode)
  (Utilities|FlowControl|Sequence
    (:then_0
      (bind _returnvalue (UserInterface|CreateWidget "/Game/Ui/New_Main_Menu.New_Main_Menu_C"))
      (UserInterface|Viewport|AddtoViewport _returnvalue 0)
      (Game|LoadStreamLevel(byName) (Utilities|Array|Get(acopy) (Variables|Default|GetStreaming_Levels) (Variables|Default|GetCurrent_Streamed_Levels)) true true)
      (Class|TTTinyTanksGameMode|SpawnPlayerTanks (Variables|Default|GetGameMode))
      (Class|TTTinyTanksGameMode|SpawnPlayerControllers (Variables|Default|GetGameMode)))))

(event EventLastManIsStanding
  (Utilities|FlowControl|Delay 1.0)
  (Class|TTTinyTanksGameMode|SetCanPlayersControlTanks (Variables|Default|GetGameMode) false)
  (CallFunction|ChangeLevel))

(fn ConstructionScript)