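; Delivery box that falls from where it is placed and spawns a TT_Pickup_BP with a random powerup on landing.
; The construction script traces downward to find the landing point, and a timeline lerps the box there.
; On landing, its sides are pushed apart with brief physics before the box destroys itself.
; A longer delayed pickup destroy is also queued, but the box's own destruction precedes it.
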(event EventBeginPlay
  (Development|PrintString (Utilities|String|ToString(Vector) (Variables|Default|GetPosition%20before%20fall)))
  (Development|PrintString (Utilities|String|ToString(Vector) (Variables|Default|GetPosition%20of%20landing)))
  (bind _fall_line (Timeline|Falling PlayFromStart)
    (:Update
      (Transformation|SetActorLocation (Math|Vector|Lerp(Vector) (Variables|Default|GetPosition%20before%20fall) (Variables|Default|GetPosition%20of%20landing) _fall_line) true false))
    (:Finished
      (bind _returnvalue (Game|SpawnActorfromClass "/Game/Blueprints/Pickups/TT_Pickup_BP.TT_Pickup_BP_C" (Math|Transform|MakeTransform (Variables|Default|GetPosition%20of%20landing) "0, 0, 0" "1,1,1") "Undefined" 0 0))
      (Utilities|FlowControl|Sequence
        (:then_0
          (Variables|/Script/TinyTanksUniProject.TT_Powerup|SetpowerupType _returnvalue (Utilities|Select :Index (Math|Random|RandomIntegerinRange 0 8) :Option%200 "PT_speedBoost" :Option%201 "PT_airblast" :Option%202 "PT_shild" :Option%203 "PT_smokeScreen" :Option%204 "PT_floating" :Option%205 "PT_fastBullet" :Option%206 "PT_missileBullet" :Option%207 "PT_stunBullet" :Option%208 "PT_undergroundBullet"))
          (Default|SetColour _returnvalue)
          (for _array_element (Variables|Default|GetAll%20Sides)
            (Physics|SetSimulatePhysics _array_element true)
            (Physics|AddForce _array_element (* (Math|Vector|GetForwardVector (Components|GetChildComponent _array_element 0)) 2e+01) "None" false))
          (Utilities|FlowControl|Delay 1.0)
          (for _array_element_2 (Variables|Default|GetAll%20Sides)
            (Physics|SetSimulatePhysics _array_element_2 false))
          (Actor|DestroyActor))
        (:then_1
          (Utilities|FlowControl|Delay 5.0)
          (Actor|DestroyActor _returnvalue))))))

(fn ConstructionScript
  (Variables|Default|SetAll%20Sides (Utilities|Array|MakeArray (Variables|Default|GetSide%201) (Variables|Default|GetSide%202) (Variables|Default|GetSide%203) (Variables|Default|GetSide%204) (Variables|Default|GetSide%206)))
  (bind _output_get (Variables|Default|SetPosition%20before%20fall (Transformation|GetActorLocation)))
  (bind _outhit (Collision|LineTraceByChannel _output_get (- _output_get "0, 0,1000.000000") "TraceTypeQuery1" false 0 "ForOneFrame"))
  (Variables|Default|SetPosition%20of%20landing (+ (.location _outhit) "0, 0,25.000000")))