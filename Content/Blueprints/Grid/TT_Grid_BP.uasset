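; Grid Blueprint that generates a flat, evenly spaced field of points on BeginPlay and visualizes it with debug spheres.
; Nested loops fill GridPoints row by row, stepping X within each row and Y between rows at a fixed height.
; A zero-length sphere trace at each point draws persistent debug shapes; hit results are unused.
; Generation is skipped if the array already holds 144 points, though the loops add 252.
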(event EventBeginPlay
  (if (== (Utilities|Array|Length (Variables|Default|GetGrid%20Points)) 144)
    (Development|PrintString "finished")
    (else
      (for _index (range 1 12)
        (if (Variables|Default|GetIs%20first%20entry)
          _
          (else
            (Variables|Default|SetCurrent%20Y%20value (+ (Variables|Default|GetCurrent%20Y%20value) 45.0))))
        (for _index_2 (range 1 21)
          (Utilities|Array|Add (Variables|Default|GetGrid%20Points) (Math|Vector|MakeVector (Variables|Default|GetCurrent%20X%20Value) (Variables|Default|GetCurrent%20Y%20value) 1e+01))
          (Variables|Default|SetCurrent%20X%20Value (+ (Variables|Default|GetCurrent%20X%20Value) 45.0)))
        (Variables|Default|SetIs%20first%20entry false)
        (Variables|Default|SetCurrent%20X%20Value -4.5e+02))
      (for _array_element (Variables|Default|GetGrid%20Points)
        (Collision|SphereTraceByChannel _array_element _array_element 22.5 "TraceTypeQuery1" false 0 "Persistent")))))

(fn ConstructionScript)