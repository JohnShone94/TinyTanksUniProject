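; Powerup holder that shows which offensive and defensive powerups its owning tank currently holds.
; UpdatePowerupHolder reads both powerups from OwningTank and sets a static mesh component for each slot.
; The offensive slot shows a super or stun missile, and the defensive slot shows a shield or floating mesh.
; A slot's mesh is cleared when it has no powerup or one of the other category.
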(event EventUpdatePowerupHolder
  (bind _deffensivepowerupmesh (Variables|Default|GetDeffensivePowerupMesh))
  (bind _offensivepowerupmesh (Variables|Default|GetOffensivePowerupMesh))
  (bind _output_get (Variables|Default|SetOffensivePowerup (Class|TTTankBase|GetCurrentOffensivePowerup (Variables|Default|GetowningTank))))
  (if (Utilities|Enum|NotEqual(Enum) _output_get "PT_none")
    (switch Utilities|FlowControl|Switch|SwitchonEPowerupType (Variables|Default|GetOffensivePowerup)
      (:PT_none
        (Components|StaticMesh|SetStaticMesh (Variables|Default|GetOffensivePowerupMesh) 0 :!label _label))
      (:PT_shild
        (goto _label))
      (:PT_floating
        (goto _label))
      (:PT_missileBullet
        (Components|StaticMesh|SetStaticMesh _offensivepowerupmesh (Variables|Default|GetSuperMissileMesh)))
      (:PT_stunBullet
        (Components|StaticMesh|SetStaticMesh _offensivepowerupmesh (Variables|Default|GetStunMissileMesh))))
    (else
      (goto _label)))
  (bind _output_get_2 (Variables|Default|SetDeffensivePowerup (Class|TTTankBase|GetCurrentDeffensivePowerup (Variables|Default|GetowningTank))))
  (if (Utilities|Enum|NotEqual(Enum) _output_get_2 "PT_none")
    (switch Utilities|FlowControl|Switch|SwitchonEPowerupType (Variables|Default|GetDeffensivePowerup)
      (:PT_none
        (Components|StaticMesh|SetStaticMesh (Variables|Default|GetDeffensivePowerupMesh) 0 :!label _label_2))
      (:PT_shild
        (Components|StaticMesh|SetStaticMesh _deffensivepowerupmesh (Variables|Default|GetShieldMesh)))
      (:PT_floating
        (Components|StaticMesh|SetStaticMesh _deffensivepowerupmesh (Variables|Default|GetFloatingMesh)))
      (:PT_missileBullet
        (goto _label_2))
      (:PT_stunBullet
        (goto _label_2)))
    (else
      (goto _label_2))))

(fn ConstructionScript)