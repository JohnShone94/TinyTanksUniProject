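; Team turret Blueprint, named for the blue team, that colors its static mesh to match the team it belongs to.
; The UpdateTankTeam event reads the turret team and applies the blue or red material to the mesh's first slot, printing a debug string for any other value.
; BeginPlay and the construction script are empty, and nothing in this Blueprint calls the update event.
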(event EventBeginPlay)

(event EventUpdateTankTeam
  (bind _returnvalue (Class|TTTankTurret|GetTurretTeam))
  (if (Utilities|Enum|Equal(Enum) _returnvalue "ST_blueTurret")
    (Rendering|Material|SetMaterial (Variables|Default|GetStaticMesh) 0 (Variables|Default|GetBlueMat))
    (elif (Utilities|Enum|Equal(Enum) _returnvalue "ST_redTurret")
      (Rendering|Material|SetMaterial (Variables|Default|GetStaticMesh) 0 (Variables|Default|GetRedMat))
      (else
        (Development|PrintString "Not a fucking clue")))))

(fn ConstructionScript)