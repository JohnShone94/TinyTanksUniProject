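; Player tank Blueprint that handles team visuals, shield and death effects, plus debug keyboard controls.
; Team updates recolour the base mesh and death explosion and set the missile class, which is the red-team missile for both teams.
; Shield events toggle the shield effect, while death shakes the camera, clears the mesh and triggers the explosion.
; Debug keys adjust GameMode tank and turret speeds, kill all tanks or restart the level.
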(event Custom|Tank%20Blows%20up
  ;[1 1 1] Tank Death
  (Camera|PlayWorldCameraShake "/Game/Blueprints/Camera/RockFall_CamShake.RockFall_CamShake_C" "0, 0, 0" 1.0 1e+05 0.0)
  (Components|StaticMesh|SetStaticMesh (Variables|Default|GettankBaseMesh) 0)
  (Components|Activation|Activate (Variables|Default|GetDeathExplosion) false))

(event EventUpdateTankTeam
  (bind _returnvalue (Class|TTTankBase|GetTankTeam))
  (if (Utilities|Enum|Equal(Enum) _returnvalue "ST_blueBase")
    (Variables|Default|SetmagicMissile "/Game/Blueprints/Players/TT_MagicMissile_TeamRed_BP.TT_MagicMissile_TeamRed_BP_C")
    (Effects|Components|ParticleSystem|SetColorParameter (Variables|Default|GetDeathExplosion) "TeamColour" "(R=0.000000,G=0.053867,B=0.895833,A=1.000000)")
    (Rendering|Material|SetMaterial (Variables|Default|GettankBaseMesh) 0 (Variables|Default|GetBlueTeamBase))
    (elif (Utilities|Enum|Equal(Enum) _returnvalue "ST_redBase")
      (Variables|Default|SetmagicMissile "/Game/Blueprints/Players/TT_MagicMissile_TeamRed_BP.TT_MagicMissile_TeamRed_BP_C")
      (Effects|Components|ParticleSystem|SetColorParameter (Variables|Default|GetDeathExplosion) "TeamColour" "(R=0.895833,G=0.000000,B=0.022960,A=1.000000)")
      (Rendering|Material|SetMaterial (Variables|Default|GettankBaseMesh) 0 (Variables|Default|GetRedTeamBase)))))

(event EventTankHasDied
  ;[1 1 1] Tank Death
  (Camera|PlayWorldCameraShake "/Game/Blueprints/Camera/RockFall_CamShake.RockFall_CamShake_C" "0, 0, 0" 1.0 1e+05 0.0)
  (Components|StaticMesh|SetStaticMesh (Variables|Default|GettankBaseMesh) 0)
  (Components|Activation|Activate (Variables|Default|GetDeathExplosion) false))

(event EventShieldActive
  (bind _shield (Variables|Default|GetShield))
  (if (Variables|Default|GetbIsShilded)
    (Components|Activation|Activate _shield false)
    (else
      (Components|Activation|Deactivate _shield))))

(event EventTankHasFired
  ;[1 1 1] Spawn muzzle flash
)

(event EventBeginPlay)

(event Input|KeyboardEvents|O
  (params (Key :type Key%20Structure :default "None"))
  (:Pressed
    (for _array_element (Variables|/Script/TinyTanksUniProject.TT_TinyTanksGameMode|GettankArray (Variables|Default|GetgameMode))
      (Class|TTTankBase|KillTank _array_element false))))

(event Input|KeyboardEvents|P
  (params (Key :type Key%20Structure :default "None"))
  (:Pressed
    (Development|ExecuteConsoleCommand "restartlevel" 0)))

(event Input|KeyboardEvents|Equals
  (params (Key :type Key%20Structure :default "None"))
  (:Pressed
    (Class|TTTinyTanksGameMode|UpdateTurretRotateSpeed (Variables|Default|GetgameMode) 0.5)))

(event Input|KeyboardEvents|Hyphen
  (params (Key :type Key%20Structure :default "None"))
  (:Pressed
    (Class|TTTinyTanksGameMode|UpdateTurretRotateSpeed (Variables|Default|GetgameMode) -0.5)))

(event Input|KeyboardEvents|9
  (params (Key :type Key%20Structure :default "None"))
  (:Pressed
    (Class|TTTinyTanksGameMode|UpdateTankRotateSpeed (Variables|Default|GetgameMode) -0.5)))

(event Input|KeyboardEvents|0
  (params (Key :type Key%20Structure :default "None"))
  (:Pressed
    (Class|TTTinyTanksGameMode|UpdateTankRotateSpeed (Variables|Default|GetgameMode) 0.5)))

(event Input|KeyboardEvents|RightBracket
  (params (Key :type Key%20Structure :default "None"))
  (:Pressed
    (Class|TTTinyTanksGameMode|UpdateTankSpeed (Variables|Default|GetgameMode) 0.5)))

(event Input|KeyboardEvents|LeftBracket
  (params (Key :type Key%20Structure :default "None"))
  (:Pressed
    (Class|TTTinyTanksGameMode|UpdateTankSpeed (Variables|Default|GetgameMode) -0.5)))

(fn ConstructionScript)