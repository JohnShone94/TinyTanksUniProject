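; Magic missile projectile Blueprint with team-coloured effects, extending a parent that supplies the bullet hit behaviour.
; When setup finishes, it sets the Niagara TeamColour parameter to blue for the blue team and green otherwise.
; On hit, it runs the parent effect, swaps the particle system's template to an explosion and unpauses the Niagara component.
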(event EventSetupFinished
  (if (Variables|Default|GetbIsBlueTeam)
    (Effects|Components|ParticleSystem|SetColorParameter (Variables|Default|GetNiagara) "TeamColour" "(R=0.000000,G=0.053867,B=0.895833,A=1.000000)")
    (else
      (Effects|Components|ParticleSystem|SetColorParameter (Variables|Default|GetNiagara) "TeamColour" "(R=0.058358,G=0.427083,B=0.000000,A=1.000000)"))))

(event EventRunBulletHitEffect
  (|CallParentFunction)
  (Effects|Components|ParticleSystem|SetTemplate (Variables|Default|GetParticleSystem) (Variables|Default|GetExplosion))
  (Class|NiagaraComponent|SetPaused (Variables|Default|GetNiagara) false))

(fn ConstructionScript)