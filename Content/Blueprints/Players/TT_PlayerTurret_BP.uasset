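; Player turret Blueprint for Tiny Tanks that shows its team's look and carries debug shortcuts.
; A team update event checks the turret's team and swaps the gun base and crystal materials to the team one or team two set.
; Gamepad special buttons and the O and P keys, gated by the game mode's debug flag, kill every tank in its tank array or restart the level.
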(event EventBeginPlay)

(event EventUpdateTankTeam
  (bind _returnvalue (Class|TTTankTurret|GetTurretTeam))
  (if (Utilities|Enum|Equal(Enum) _returnvalue "ST_teamOneTurret")
    (Rendering|Material|SetMaterial (Variables|Default|GettankGunBase) 0 (Variables|Default|GetTeamOneTurretMaterial))
    (Rendering|Material|SetMaterial (Variables|Default|GetCrystal) 0 (Variables|Default|GetTeamOneCrystalMaterial))
    (elif (Utilities|Enum|Equal(Enum) _returnvalue "ST_teamTwoTurret")
      (Rendering|Material|SetMaterial (Variables|Default|GettankGunBase) 0 (Variables|Default|GetTeamTwoTurretMaterial))
      (Rendering|Material|SetMaterial (Variables|Default|GetCrystal) 0 (Variables|Default|GetTeamTwoCrystalMaterial)))))

(event Input|KeyboardEvents|O
  (params (Key :type Key%20Structure :default "None"))
  ;[1 1 1] Move to next level / Reset game
  (:Pressed
    (bind _astt_tiny_tanks_game_mode (Utilities|Casting|CastToTT_TinyTanksGameMode (Game|GetGameMode)))
    (if (Variables|/Script/TinyTanksUniProject.TT_TinyTanksGameMode|GetbDebugActive _astt_tiny_tanks_game_mode)
      (for _array_element (Variables|/Script/TinyTanksUniProject.TT_TinyTanksGameMode|GettankArray _astt_tiny_tanks_game_mode)
        (Class|TTTankBase|KillTank _array_element false)))))

(event Input|KeyboardEvents|P
  (params (Key :type Key%20Structure :default "None"))
  ;[1 1 1] Move to next level / Reset game
  (:Pressed
    (bind _astt_tiny_tanks_game_mode (Utilities|Casting|CastToTT_TinyTanksGameMode (Game|GetGameMode)))
    (if (Variables|/Script/TinyTanksUniProject.TT_TinyTanksGameMode|GetbDebugActive _astt_tiny_tanks_game_mode)
      (Development|ExecuteConsoleCommand "restartlevel" 0))))

(event Input|GamepadEvents|GamepadSpecialLeft
  (params (Key :type Key%20Structure :default "None"))
  ;[1 1 1] Move to next level / Reset game
  (:Pressed
    (bind _astt_tiny_tanks_game_mode (Utilities|Casting|CastToTT_TinyTanksGameMode (Game|GetGameMode)))
    (if (Variables|/Script/TinyTanksUniProject.TT_TinyTanksGameMode|GetbDebugActive _astt_tiny_tanks_game_mode)
      (Development|ExecuteConsoleCommand "restartlevel" 0))))

(event Input|GamepadEvents|GamepadSpecialRight
  (params (Key :type Key%20Structure :default "None"))
  ;[1 1 1] Move to next level / Reset game
  (:Pressed
    (bind _astt_tiny_tanks_game_mode (Utilities|Casting|CastToTT_TinyTanksGameMode (Game|GetGameMode)))
    (if (Variables|/Script/TinyTanksUniProject.TT_TinyTanksGameMode|GetbDebugActive _astt_tiny_tanks_game_mode)
      (for _array_element (Variables|/Script/TinyTanksUniProject.TT_TinyTanksGameMode|GettankArray _astt_tiny_tanks_game_mode)
        (Class|TTTankBase|KillTank _array_element false)))))

(fn ConstructionScript)