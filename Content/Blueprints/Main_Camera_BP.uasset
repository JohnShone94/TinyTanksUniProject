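; Main camera actor that moves from its menu view to a fixed, downward-angled game view.
; The transition runs automatically after a short delay on BeginPlay, or immediately when the Movetogameview event is called.
; It captures the current transform, then a timeline alpha lerps location and rotation to hardcoded targets, taking the shortest rotation path.
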(event Custom|Move%20to%20game%20view
  (Variables|Default|SetMenu_View (Transformation|GetActorLocation))
  (Variables|Default|SetMenu_Rotation (Transformation|GetActorRotation))
  (bind _change_location (Timeline|Game%20view%20timeline PlayFromStart)
    (:Update
      (Transformation|SetActorLocationAndRotation (Math|Vector|Lerp(Vector) (Variables|Default|GetMenu_View) "0,228.000000,593.869995" _change_location) (Math|Rotator|Lerp(Rotator) (Variables|Default|GetMenu_Rotation) "-70.000000,-90.000000, 0" _change_location true)))))

(event EventBeginPlay
  (Utilities|FlowControl|Delay 2.0)
  (Variables|Default|SetMenu_View (Transformation|GetActorLocation))
  (Variables|Default|SetMenu_Rotation (Transformation|GetActorRotation))
  (bind _change_location (Timeline|Game%20view%20timeline PlayFromStart)
    (:Update
      (Transformation|SetActorLocationAndRotation (Math|Vector|Lerp(Vector) (Variables|Default|GetMenu_View) "0,228.000000,593.869995" _change_location) (Math|Rotator|Lerp(Rotator) (Variables|Default|GetMenu_Rotation) "-70.000000,-90.000000, 0" _change_location true)))))

(event Collision|EventActorBeginOverlap
  (params (OtherActor :type Actor%20Object%20Reference)))

(event EventTick
  (params (DeltaSeconds :type Float%20%28single-precision%29)))

(fn ConstructionScript)