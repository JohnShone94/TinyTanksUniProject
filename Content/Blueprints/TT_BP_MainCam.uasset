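; Main camera actor for Tiny Tanks that animates between menu, gameplay and level-transition views using timeline-driven position and rotation lerps.
; On BeginPlay or Setviewtogameview, it waits briefly, glides from menu to game view, then enables tank control through the game mode.
; Changelevel disables control, moves to the transition view, jumps to a post-teleport position, glides back to game view and re-enables control.
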(event Custom|Change%20level
  (bind _astt_tiny_tanks_game_mode (Utilities|Casting|CastToTT_TinyTanksGameMode (Game|GetGameMode)))
  (Class|TTTinyTanksGameMode|SetCanPlayersControlTanks _astt_tiny_tanks_game_mode false)
  (bind _change_location (Timeline|Transition%20levels PlayFromStart)
    (:Update
      (Transformation|SetActorTransform (Math|Transform|MakeTransform (Math|Vector|Lerp(Vector) (Variables|Default|GetGame_view_Position) (Variables|Default|GetTransition_Position_Pre_TP) _change_location) (Math|Rotator|Lerp(Rotator) (Variables|Default|GetGame_Rotation) (Variables|Default|GetTransition_Rotation) _change_location) "1,1,1")))
    (:Finished
      (Transformation|SetActorLocation (Variables|Default|GetTransition_Position_Post_TP) false false)
      (bind _change_location_2 (Timeline|Timeline_2 PlayFromStart)
        (:Update
          (Transformation|SetActorTransform (Math|Transform|MakeTransform (Math|Vector|Lerp(Vector) (Variables|Default|GetTransition_Position_Post_TP) (Variables|Default|GetGame_view_Position) _change_location_2) (Math|Rotator|Lerp(Rotator) (Variables|Default|GetTransition_Rotation) (Variables|Default|GetGame_Rotation) _change_location_2) "1,1,1")))
        (:Finished
          (bind _astt_tiny_tanks_game_mode_2 (Utilities|Casting|CastToTT_TinyTanksGameMode (Game|GetGameMode)))
          (Class|TTTinyTanksGameMode|SetCanPlayersControlTanks _astt_tiny_tanks_game_mode_2 true))))))

(event Custom|Set%20view%20to%20game%20view
  (Utilities|FlowControl|Delay 2.0)
  (bind _change_location (Timeline|Move%20to%20Main%20view PlayFromStart)
    (:Update
      (Transformation|SetActorLocationAndRotation (Math|Vector|Lerp(Vector) (Variables|Default|GetMenu_View_Position) (Variables|Default|GetGame_view_Position) _change_location) (Math|Rotator|Lerp(Rotator) (Variables|Default|GetMenu_Rotation) (Variables|Default|GetGame_Rotation) _change_location true)))
    (:Finished
      (bind _astt_tiny_tanks_game_mode (Utilities|Casting|CastToTT_TinyTanksGameMode (Game|GetGameMode)))
      (Class|TTTinyTanksGameMode|SetCanPlayersControlTanks _astt_tiny_tanks_game_mode true))))

(event EventBeginPlay
  (Utilities|FlowControl|Delay 2.0)
  (bind _change_location (Timeline|Move%20to%20Main%20view PlayFromStart)
    (:Update
      (Transformation|SetActorLocationAndRotation (Math|Vector|Lerp(Vector) (Variables|Default|GetMenu_View_Position) (Variables|Default|GetGame_view_Position) _change_location) (Math|Rotator|Lerp(Rotator) (Variables|Default|GetMenu_Rotation) (Variables|Default|GetGame_Rotation) _change_location true)))
    (:Finished
      (bind _astt_tiny_tanks_game_mode (Utilities|Casting|CastToTT_TinyTanksGameMode (Game|GetGameMode)))
      (Class|TTTinyTanksGameMode|SetCanPlayersControlTanks _astt_tiny_tanks_game_mode true))))

(fn ConstructionScript)