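; A PVE hazard tile that counts down, then drops away and destroys itself.
; The countdown starts after a random delay at BeginPlay or when a tank overlaps its Box.
; A DoN loop ticks on short delays, resetting if the tank's exit has cleared ShouldFall.
; On the final count, the tile simulates physics, gets a random angular impulse, loses collision and is later destroyed.
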(event OnComponentBeginOverlap(Box)
  (params (OverlappedComponent :type Primitive%20Component%20Object%20Reference) (OtherActor :type Actor%20Object%20Reference) (OtherComp :type Primitive%20Component%20Object%20Reference) (OtherBodyIndex :type Integer) (bFromSweep :type Boolean) (SweepResult :type Hit%20Result%20Structure%20%28by%20ref%29))
  (if (not (Variables|Default|GetIs%20falling))
    (Utilities|Casting|CastToTT_TankBase OtherActor)
    (Variables|Default|SetShould%20Fall? true)
    (Utilities|FlowControl|DoOnce false
      (:Completed
        (CallFunction|Fall)))))

(event OnComponentEndOverlap(Box)
  (params (OverlappedComponent :type Primitive%20Component%20Object%20Reference) (OtherActor :type Actor%20Object%20Reference) (OtherComp :type Primitive%20Component%20Object%20Reference) (OtherBodyIndex :type Integer))
  (if (not (Variables|Default|GetIs%20falling))
    (Utilities|Casting|CastToTT_TankBase OtherActor)
    (Variables|Default|SetShould%20Fall? false)))

(event Custom|Fall
  (bind _colision (Variables|Default|GetColision))
  (bind _counter (Utilities|FlowControl|DoN 4 :!label _label)
    (:Exit
      (if (== _counter 4)
        (Variables|Default|SetIs%20falling true)
        (Physics|SetSimulatePhysics _colision true)
        (Utilities|FlowControl|Delay 0.5)
        (Class|PrimitiveComponent|AddAngularImpulseinDegrees _colision (+ (Utilities|Select :Index (Math|Random|RandomIntegerinRange 0 2) :Option%200 "300.000000, 0, 0" :Option%201 "0,300.000000, 0" :Option%202 "0, 0,300.000000") (Utilities|Select :Index (Math|Random|RandomIntegerinRange 0 2) :Option%200 "300.000000, 0, 0" :Option%201 "0,300.000000, 0" :Option%202 "0, 0,300.000000")) "None" false)
        (Collision|SetActorEnableCollision false)
        (Utilities|FlowControl|Delay 3.0)
        (Actor|DestroyActor)
        (else
          (Utilities|FlowControl|Delay 0.75)
          (if (Variables|Default|GetShould%20Fall?)
            (goto _label)
            (else
              (CallFunction|StopFall))))))))

(event Custom|Reset%20fall
  (bind _colision (Variables|Default|GetColision))
  (Utilities|FlowControl|Sequence
    (:then_0
      (Utilities|FlowControl|DoOnce false) ; enters at Reset
    )
    (:then_1
      (Utilities|FlowControl|DoN 4) ; enters at Reset
    )))

(event Custom|Stop%20fall
  (CallFunction|ResetFall))

(event EventBeginPlay
  (Utilities|FlowControl|Delay (Math|Random|RandomFloatinRange 0.0 3.0))
  (Utilities|FlowControl|Sequence
    (:then_0
      (Variables|Default|SetShould%20Fall? true)
      (Utilities|FlowControl|DoOnce false
        (:Completed
          (CallFunction|Fall))))))

(fn ConstructionScript)