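; Spike trap tile for the PVE danger set that kills any tank overlapping its DamageBox.
; Unless flagged TriggeredByButton, a RiseBox overlap waits briefly, then a timeline raises and lowers the DamageBox, locked by SpikesAreMoving until finished.
; SpikesAreMoving is set before the tank cast, so a non-tank overlap leaves the trap locked.
; ButtonPressed plays a separate raise-only timeline between the same endpoints, computed in the construction script.
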(event OnComponentBeginOverlap(Damagebox)
  (params (OverlappedComponent :type Primitive%20Component%20Object%20Reference) (OtherActor :type Actor%20Object%20Reference) (OtherComp :type Primitive%20Component%20Object%20Reference) (OtherBodyIndex :type Integer) (bFromSweep :type Boolean) (SweepResult :type Hit%20Result%20Structure%20%28by%20ref%29))
  (bind _astt_tank_base (Utilities|Casting|CastToTT_TankBase OtherActor))
  (Class|TTTankBase|KillTank _astt_tank_base))

(event OnComponentBeginOverlap(Risebox)
  (params (OverlappedComponent :type Primitive%20Component%20Object%20Reference) (OtherActor :type Actor%20Object%20Reference) (OtherComp :type Primitive%20Component%20Object%20Reference) (OtherBodyIndex :type Integer) (bFromSweep :type Boolean) (SweepResult :type Hit%20Result%20Structure%20%28by%20ref%29))
  (if (not (Variables|Default|GetTriggered%20by%20button?))
    (Utilities|FlowControl|Delay 1.5)
    (if (not (Variables|Default|GetSpikes%20are%20moving?))
      (Variables|Default|SetSpikes%20are%20moving? true)
      (Utilities|Casting|CastToTT_TankBase OtherActor)
      (CallFunction|RiseandLowerSpikes))))

(event Custom|Rise%20and%20lower%20spikes
  (bind _move_spikes (Timeline|Rise%20Spikes%20then%20lower PlayFromStart)
    (:Update
      (Transformation|SetWorldLocation (Variables|Default|GetDamage%20box) (Math|Vector|Lerp(Vector) (Variables|Default|GetStart%20Location) (Variables|Default|GetEnd%20Location) _move_spikes) false false))
    (:Finished
      (Variables|Default|SetSpikes%20are%20moving? false))))

(event Custom|Button%20Pressed]
  (bind _move_spikes (Timeline|Raise%20Spikes PlayFromStart)
    (:Update
      (Transformation|SetWorldLocation (Variables|Default|GetDamage%20box) (Math|Vector|Lerp(Vector) (Variables|Default|GetStart%20Location) (Variables|Default|GetEnd%20Location) _move_spikes) false false))))

(fn ConstructionScript
  (bind _output_get (Variables|Default|SetStart%20Location (Transformation|GetWorldLocation (Variables|Default|GetDamage%20box))))
  (Variables|Default|SetEnd%20Location (+ _output_get "0, 0,40.000000")))